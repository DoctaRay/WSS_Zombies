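; BP_Zombie is an AI enemy that damages the player on contact.
; On BeginPlay it runs the BT_AdvancedAI behavior tree and sets the TargetDestination blackboard key to the zero vector.
; Every Tick it looks up the first Player actor and, while its capsule overlaps that actor, applies fixed damage each frame with no cooldown.
; A capsule sphere trace and debug prints are left unconnected.
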(event `self.ReceiveBeginPlay`
  (`AIController.RunBehaviorTree` (`AIBlueprintHelperLibrary.GetAIController` self) "/Game/AdvancedAI/BT_AdvancedAI.BT_AdvancedAI")
  (`BlackboardComponent.SetValueAsVector` (`AIBlueprintHelperLibrary.GetBlackboard` self) "TargetDestination" (0.0 0.0 0.0)))

(event `self.ReceiveTick`
  (params (DeltaSeconds :type "Float (single-precision)"))
  (bind _outactors (`GameplayStatics.GetAllActorsOfClass` "/Game/Player.Player_C"))
  (bind _output (`|GetArrayItem` _outactors))
  (if (`PrimitiveComponent.IsOverlappingActor` (`self.CapsuleComponent`) _output)
    (bind _returnvalue (`GameplayStatics.ApplyDamage` _output 10.0 (`self.GetInstigatorController`) self "/Script/Engine.DamageType"))))

(fn `UserConstructionScript`)