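; BP_PowerUpAmmoFill is a power-up that restocks one of the player's weapons when activated.
; OnActivated takes the first Player actor in the world and uses IsPrimaryWeapon to pick the second attached actor if true, otherwise the first.
; It casts that actor to SWeapon, calls StockUp and destroys itself, relying on attachment order to identify the weapon.
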(event `self.OnActivated`
  (bind _outactors (`GameplayStatics.GetAllActorsOfClass` "/Game/Player.Player_C"))
  (bind _output (`|GetArrayItem` _outactors))
  (bind _children (`/DatasmithContent/Blueprints/FBXImporter/FBXImporterUtils.GetAllAttachedActors` _output))
  (if (`SCharacter.bIsPrimaryWeapon` _output)
    (bind _assweapon (cast `SWeapon` (`|GetArrayItem` _children 1)))
    (`SWeapon.StockUp` _assweapon)
    (`self.K2_DestroyActor`)
    (else
      (bind _assweapon_2 (cast `SWeapon` (`|GetArrayItem` _children)))
      (`SWeapon.StockUp` _assweapon_2)
      (`self.K2_DestroyActor`))))

(fn `UserConstructionScript`)