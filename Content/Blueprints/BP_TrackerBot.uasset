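; BP_TrackerBot is a bot that chases the player pawn by pushing its mesh with physics forces.
; FindNextPath runs a synchronous navigation query to the player and returns the second path point, or the bot's own location if none exists.
; Tick applies force toward that point as a velocity change, repathing and printing a debug string once within the required distance.
; Debug arrow and sphere drawing are present but unconnected.
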(event `self.ReceiveBeginPlay`
  (bind _fvector (`self.FindNextPath`))
  (set `self.NextPathPoint` _fvector)
  (set `self.bUseVelocityChange` true))

(event `self.ReceiveTick`
  (params (DeltaSeconds :type "Float (single-precision)"))
  ;[1 1 1] Finding Next Path Point of Tracker Bot
  (bind _output_get (set `self.DistanceToTarget` (`KismetMathLibrary.VSize` (- (`self.K2_GetActorLocation`) (`self.NextPathPoint`)))))
  (if (<= _output_get (`self.RequiredDistanceToTarget`))
    (bind _fvector (`self.FindNextPath`))
    (bind _output_get_2 (set `self.NextPathPoint` _fvector))
    (`KismetSystemLibrary.DrawDebugString` _output_get_2 "Target Reached!" null)
    (else
      (bind _output_get_3 (set `self.ForceDirection` (- (`self.NextPathPoint`) (`self.K2_GetActorLocation`))))
      (`PrimitiveComponent.AddForce` (`self.MeshComp`) (* (`KismetMathLibrary.Normal` _output_get_3) (`self.MovementForce`)) "None" (`self.bUseVelocityChange`)))))

(fn `FindNextPath`
  (returns (FVector :type "Vector Structure"))
  (bind _returnvalue (`NavigationSystemV1.FindPathToActorSynchronously` (`self.K2_GetActorLocation`) (`GameplayStatics.GetPlayerPawn` 0) 50.0 null null))
  (bind _pathpoints (`NavigationPath.PathPoints` _returnvalue))
  (if (> (`KismetArrayLibrary.Array_Length` _pathpoints) 1)
    (return (`|GetArrayItem` _pathpoints 1))
    (else
      (return (`self.K2_GetActorLocation`)))))

(fn `UserConstructionScript`)