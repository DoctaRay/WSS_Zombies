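; Player Blueprint that sets up the HUD and handles switching between two cameras.
; BeginPlay creates the Crosshair and HealthIndicator_BP widgets and adds both to the viewport.
; The FP_Cam input drives a FlipFlop: one press activates FPCam and deactivates CameraComp, the next reactivates CameraComp.
; The node that would deactivate FPCam is unconnected, so FPCam stays active after switching back.
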(event `self.ReceiveBeginPlay`
  (`|ExecutionSequence`
    (:`then_0`
      (bind _returnvalue (`|CreateWidget` "/Game/UI/Crosshair.Crosshair_C"))
      (`UserWidget.AddToViewport` _returnvalue 0))
    (:`then_1`
      (bind _returnvalue_2 (`|CreateWidget` "/Game/UI/HealthIndicator_BP.HealthIndicator_BP_C"))
      (`UserWidget.AddToViewport` _returnvalue_2 0))))

(event `InputAction|FP_Cam`
  (params (Key :type "Key Structure"))
  (:`Pressed`
    (`/Engine/EditorBlueprintResources/StandardMacros.FlipFlop`
      (:`A`
        (`ActorComponent.SetActive` (`self.FP_Cam`) true false)
        (`ActorComponent.SetActive` (`self.CameraComp`) false true))
      (:`B`
        (`ActorComponent.SetActive` (`self.CameraComp`) true false)))))

(fn `UserConstructionScript`)